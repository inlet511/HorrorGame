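; BP_HorrorHUD creates the horror game's on-screen UI and a simple touch UI through two custom events.
; CreateHorrorUI creates and adds UI_Horror if no valid instance exists, then passes player 0's BP_HorrorCharacter to its SetupCharacter.
; CreateTouchSimpleUI reuses or creates UI_TouchSimple and adds it to the player screen on every call.
; BeginPlay and Tick are empty, so neither widget appears until its event is called.
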(event Custom|CreateHorrorUI
  (Utilities|IsValid (Variables|Default|GetHorrorUI)
    (:Is%20Valid
      _)
    (:Is%20Not%20Valid
      (bind _returnvalue (UserInterface|CreateWidget "/Game/UMG/UI_Horror.UI_Horror_C"))
      (bind _output_get (Variables|Default|SetHorrorUI _returnvalue))
      (UserInterface|Viewport|AddtoPlayerScreen _output_get)))
  (bind _asbp_horror_character (Utilities|Casting|CastToBP_HorrorCharacter (Game|GetPlayerCharacter 0)))
  (Default|SetupCharacter _output_get _asbp_horror_character))

(event Custom|CreateTouchSimpleUI
  (Utilities|IsValid (Variables|Default|GetTouchSampleUI)
    (:Is%20Valid
      _)
    (:Is%20Not%20Valid
      (bind _returnvalue (UserInterface|CreateWidget "/Game/Input/Touch/UI_TouchSimple.UI_TouchSimple_C"))
      (Variables|Default|SetTouchSampleUI _returnvalue)))
  (UserInterface|Viewport|AddtoPlayerScreen (Variables|Default|GetTouchSampleUI)))

(event EventBeginPlay)

(event Collision|EventActorBeginOverlap
  (params (OtherActor :type Actor%20Object%20Reference)))

(event EventTick
  (params (DeltaSeconds :type Float%20%28single-precision%29)))

(fn ConstructionScript)