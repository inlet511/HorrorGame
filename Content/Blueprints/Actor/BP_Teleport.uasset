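; BP_Teleport is a one-way box trigger that seamlessly moves BP_FirstPersonCharacter to a paired BP_Teleport.
; An entrance finds its exit by its first tag plus "End", and exits never send.
; Location is carried over relative to both transforms; Reverse also turns position, control rotation and velocity 180° through helper functions, otherwise world velocity is kept.
; A DoOnce with a short delayed reset debounces overlaps.
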(event OnComponentBeginOverlap(Box)
  (params (OverlappedComponent :type Primitive%20Component%20Object%20Reference) (OtherActor :type Actor%20Object%20Reference) (OtherComp :type Primitive%20Component%20Object%20Reference) (OtherBodyIndex :type Integer) (bFromSweep :type Boolean) (SweepResult :type Hit%20Result%20Structure%20%28by%20ref%29))
  (bind _returnvalue (Game|GetPlayerController 0))
  (Utilities|FlowControl|DoOnce false :!label _label
    (:Completed
      (Utilities|FlowControl|Sequence
        (:then_0
          (if (not (Utilities|String|Contains (Utilities|String|ToString(Name) (Utilities|Array|Get(acopy) (Variables|Actor|GetTags))) "End" false true))
            (bind _asbp_first_person_character (Utilities|Casting|CastToBP_FirstPersonCharacter OtherActor))
            (bind _outactors (Actor|GetAllActorsOfClasswithTag "BP_Teleport_C" (Utilities|String|StringToName (Utilities|String|Append (Utilities|String|ToString(Name) (Utilities|Array|Get(acopy) (Variables|Actor|GetTags))) "End"))))
            (Utilities|IsValid (Utilities|Array|Get(acopy) _outactors)
              (:Is%20Valid
                (if (Variables|Default|GetReverse)
                  (Transformation|SetActorLocation _asbp_first_person_character (CallFunction|InverseLocation (Transformation|GetActorTransform (Utilities|Array|Get(acopy) _outactors)) (Transformation|GetActorLocation _asbp_first_person_character)) false false)
                  (Pawn|SetControlRotation _returnvalue (CallFunction|InverseRotation (Transformation|GetActorTransform (Utilities|Array|Get(acopy) _outactors)) (Pawn|GetControlRotation _returnvalue :!class /Script/Engine.Controller)))
                  (Variables|/Script/Engine.MovementComponent|SetVelocity (Variables|/Script/Engine.Character|GetCharacterMovement _asbp_first_person_character) (CallFunction|InverseVelocity (Transformation|GetActorTransform (Utilities|Array|Get(acopy) _outactors)) (Transformation|GetVelocity _asbp_first_person_character)))
                  (else
                    (Transformation|SetActorLocation _asbp_first_person_character (Math|Transform|TransformLocation (Transformation|GetActorTransform (Utilities|Array|Get(acopy) _outactors)) (Math|Transform|InverseTransformLocation (Transformation|GetActorTransform) (Transformation|GetActorLocation _asbp_first_person_character))) false false)
                    (Variables|/Script/Engine.MovementComponent|SetVelocity (Variables|/Script/Engine.Character|GetCharacterMovement _asbp_first_person_character) (Transformation|GetVelocity _asbp_first_person_character))))))))
        (:then_1
          (Utilities|FlowControl|Delay 0.1)
          (goto _label Reset))))))

(event EventBeginPlay)

(event Collision|EventActorBeginOverlap
  (params (OtherActor :type Actor%20Object%20Reference)))

(event EventTick
  (params (DeltaSeconds :type Float%20%28single-precision%29)))

(fn ConstructionScript
  (Components|Box|SetBoxExtent (Variables|Default|GetBox) (Variables|Default|GetInitBoxExtent) true))

(fn InverseVelocity
  (params (EndTransform :type Transform%20%28by%20ref%29) (Velocity :type Vector))
  (return (Math|Transform|TransformDirection EndTransform (Math|Vector|RotateVector (Math|Transform|InverseTransformDirection (Transformation|GetActorTransform) Velocity) "0.000000,180.000000,0.000000"))))

(fn InverseRotation
  (params (EndTransform :type Transform%20%28by%20ref%29) (Rotation :type Rotator))
  (return (Math|Transform|TransformRotation EndTransform (Math|Rotator|CombineRotators (Math|Transform|InverseTransformRotation (Transformation|GetActorTransform) Rotation) "0.000000,180.000000,0.000000"))))

(fn InverseLocation
  (params (EndTransform :type Transform%20%28by%20ref%29) (Location :type Vector))
  (bind _returnvalue (Transformation|GetActorTransform))
  (bind _returnvalue_2 (Math|Transform|InverseTransformLocation _returnvalue Location))
  (bind (_x _y _z) (Math|Vector|BreakVector _returnvalue_2))
  (return (Math|Transform|TransformLocation EndTransform (Math|Vector|MakeVector (* _x -1.0) (* _y -1.0) _z))))